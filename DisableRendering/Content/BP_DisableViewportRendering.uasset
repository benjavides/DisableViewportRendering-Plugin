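; Actor that turns off main viewport rendering at play start, exposing events to enable or disable it again.
; When disabling on play, it can first gather every SceneCapture2D actor in the level.
; While viewport rendering is off, Tick can manually call CaptureScene on each gathered capture so render targets keep updating.
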(event Custom|DisableViewportRendering
  (Class|DisableRenderingBPLibrary|SetViewportRenderingEnabled false)
  (Variables|Default|SetRenderingEnabled? false))

(event Custom|EnableViewportRendering
  (Class|DisableRenderingBPLibrary|SetViewportRenderingEnabled true)
  (Variables|Default|SetRenderingEnabled? true))

(event EventBeginPlay
  (if (Variables|Default|GetDisableOnPlay)
    (Utilities|FlowControl|Sequence
      (:then_0
        (if (Variables|Default|GetFindSceneCapture2Ds)
          (bind _outactors (Actor|GetAllActorsOfClass "/Script/Engine.SceneCapture2D"))
          (Variables|Default|SetSceneCaptures _outactors)))
      (:then_1
        (CallFunction|DisableViewportRendering)))))

(event EventTick
  (params (DeltaSeconds :type Float%20%28single-precision%29))
  (if (and (not (Variables|Default|GetRenderingEnabled?)) (Variables|Default|GetTickSceneCaptures))
    (for _array_element (Variables|Default|GetSceneCaptures)
      (Rendering|SceneCapture|CaptureScene (Variables|/Script/Engine.SceneCapture2D|GetCaptureComponent2D _array_element) :!class /Script/Engine.SceneCaptureComponent2D))))

(fn ConstructionScript)